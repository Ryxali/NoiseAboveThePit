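; Audio manager that drives the main theme and triggers announcer-style sounds from the player's combo multiplier and life.
; Each Tick it feeds the multiplier into MainTheme's "Combo" parameter and plays a sound at set milestones, switching to a MaxCombo check at the top tier and regular intervals beyond.
; At zero life it plays Death, though this check is skipped while a milestone sound is already playing at its threshold.
; IsPlaying guards prevent overlapping restarts.
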(event `self.ReceiveBeginPlay`)

(event `self.ReceiveActorBeginOverlap`
  (params (OtherActor :type "Actor Object Reference")))

(event `self.ReceiveTick`
  (params (DeltaSeconds :type "Float (single-precision)"))
  (bind _death (`self.Death`))
  (bind _returnvalue (`GameHUD.GetComboMultiplyer`))
  (`FMODAudioComponent.SetParameter` (`self.MainTheme`) "Combo" (`KismetStringLibrary.Conv_StringToDouble` _returnvalue))
  (bind _returnvalue_2 (`KismetStringLibrary.Conv_StringToInt` _returnvalue))
  (if (== _returnvalue_2 5)
    (bind _returnvalue_3 (`FMODAudioComponent.IsPlaying` :!label _label))
    (if (not _returnvalue_3)
      (`FMODAudioComponent.Play`)
      (bind _returnvalue_4 (`GameHUD.GetLife` :!label _label_2))
      (if (== (`KismetStringLibrary.Conv_StringToInt` _returnvalue_4) 0)
        (bind _returnvalue_5 (`FMODAudioComponent.IsPlaying` _death))
        (if (not _returnvalue_5)
          (`FMODAudioComponent.Play` _death))))
    (elif (== _returnvalue_2 10)
      (goto _label)
      (elif (== _returnvalue_2 25)
        (goto _label)
        (elif (== _returnvalue_2 50)
          (goto _label)
          (elif (== _returnvalue_2 100)
            (goto _label)
            (else
              (if (== _returnvalue_2 250)
                _
                (elif (> _returnvalue_2 250)
                  (if (== (mod (- _returnvalue_2 250) 100) 0)
                    _
                    (else
                      (goto _label_2)))
                  (else
                    (goto _label_2))))
              (bind _returnvalue_6 (`FMODAudioComponent.IsPlaying` (`self.MaxCombo`)))
              (if (not _returnvalue_6)
                (`FMODAudioComponent.Play`)
                (goto _label_2)))))))))

(fn `UserConstructionScript`)