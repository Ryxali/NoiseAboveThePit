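; FloatingContainer is an actor that drifts upward and removes itself once it rises too high.
; Each tick, MoveUpwards applies a frame-rate-independent local Z offset scaled by Speed, without sweeping for collision.
; RemoveIfOutOfBounds then destroys the actor when its world Z exceeds DespawnHeight.
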(event `self.ReceiveBeginPlay`)

(event `self.ReceiveActorBeginOverlap`
  (params (OtherActor :type "Actor Object Reference")))

(event `self.ReceiveTick`
  (params (DeltaSeconds :type "Float (single-precision)"))
  (`self.Move Upwards` DeltaSeconds)
  (`self.Remove If Out Of Bounds`))

(fn `Move Upwards`
  (params (`Delta Seconds` :type "Float (double-precision)" :default 0.0))
  (`self.K2_AddActorLocalOffset` (* (0.0 0.0 1.0) (* `Delta Seconds` (`self.Speed`)))))

(fn `Remove If Out Of Bounds`
  (if (> (.z (`self.K2_GetActorLocation`)) (`self.DespawnHeight`))
    (`self.K2_DestroyActor`)))

(fn `UserConstructionScript`)